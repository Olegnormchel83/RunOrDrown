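; BP_RODHUD is the Run or Drown HUD Blueprint that decides which top-level screen to show.
; On BeginPlay it checks the current level name and adds the main menu widget when the level is MainMenu.
; In other levels it binds to the player character's OnDeath event and adds the death screen widget when the player dies.
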(event `self.ReceiveBeginPlay`
  (bind _returnvalue (`GameplayStatics.GetCurrentLevelName` true))
  (if (`KismetStringLibrary.EqualEqual_StrStr` _returnvalue "MainMenu")
    (bind _returnvalue_2 (`|CreateWidget` "/Game/RunOrDrown/UI/Menu/WBP_MainMenu.WBP_MainMenu_C"))
    (`UserWidget.AddToViewport` _returnvalue_2 0)
    (else
      (bind _asbp_rodplayer_character (cast `/Game/RunOrDrown/Blueprints/Character/BP_RODPlayerCharacter` (`GameplayStatics.GetPlayerCharacter` 0)))
      (add `/Game/RunOrDrown/Blueprints/Character/BP_RODPlayerCharacter.OnDeath` _asbp_rodplayer_character (delegate `OnPlayerDeath`)))))

(event `OnPlayerDeath`
  (bind _returnvalue (`|CreateWidget` "/Game/RunOrDrown/UI/Menu/WBP_DeathScreen.WBP_DeathScreen_C"))
  (`UserWidget.AddToViewport` _returnvalue 0))

(fn `UserConstructionScript`)