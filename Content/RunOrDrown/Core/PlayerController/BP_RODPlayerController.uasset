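; Player controller for Run Or Drown that drives the player character through Enhanced Input and manages the pause menu.
; On BeginPlay it adds the input mapping context, caches the controlled character and binds to the lake character's disappeared event to play a camera shake.
; Input actions handle camera-relative movement, look and jump.
; The pause action toggles game pause, the cursor and a reused pause widget.
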(event `self.ReceiveBeginPlay`
  (`WidgetBlueprintLibrary.SetInputMode_GameOnly` self)
  (set `self.bShowMouseCursor` false)
  (`EnhancedInputSubsystemInterface.AddMappingContext` (subsystem `EnhancedInputLocalPlayerSubsystem`) "/Game/RunOrDrown/Core/EnhancedInput/IMC_ROD.IMC_ROD" 0 (struct))
  (bind _asbp_rodplayer_character (cast `/Game/RunOrDrown/Blueprints/Character/BP_RODPlayerCharacter` (`self.K2_GetPawn`)))
  (bind _output_get (set `self.RODPlayer Character` _asbp_rodplayer_character))
  (set `self.Character Movement` (`Character.CharacterMovement` _output_get))
  (bind _returnvalue (`GameplayStatics.GetActorOfClass` "/Game/RunOrDrown/Blueprints/Character/BP_RODLakeCharacter.BP_RODLakeCharacter_C"))
  (`/Engine/EditorBlueprintResources/StandardMacros.IsValid` _returnvalue
    (:`Is Valid`
      (add `/Game/RunOrDrown/Blueprints/Character/BP_RODLakeCharacter.OnDesappeared` _returnvalue (delegate `PlayerOnTheLake`)))))

(event `PlayerOnTheLake`
  (`self.ClientStartCameraShake` "/Game/RunOrDrown/Blueprints/CameraShake/BP_CameraShake.BP_CameraShake_C" 2.0))

(event `EnhancedInput|/Game/RunOrDrown/Core/EnhancedInput/Actions/IA_RODMove`
  (params (ActionValue :type "Vector2D Structure") (ElapsedSeconds :type "Float (double-precision)") (TriggeredSeconds :type "Float (double-precision)") (InputAction :type "InputAction Object Reference" :default "/Game/RunOrDrown/Core/EnhancedInput/Actions/IA_RODMove.IA_RODMove"))
  (bind (_returnvalue_roll _returnvalue_pitch _returnvalue_yaw) (`KismetMathLibrary.BreakRotator` (`self.GetControlRotation`)))
  (bind (_returnvalue_roll_2 _returnvalue_pitch_2 _returnvalue_yaw_2) (`KismetMathLibrary.BreakRotator` (`self.GetControlRotation`)))
  (:`Triggered`
    (`Pawn.AddMovementInput` (`self.RODPlayer Character`) (`KismetMathLibrary.GetRightVector` (`KismetMathLibrary.MakeRotator` _returnvalue_roll_2 0.0 _returnvalue_yaw_2)) ActionValue_X false)
    (`Pawn.AddMovementInput` (`self.RODPlayer Character`) (`KismetMathLibrary.GetForwardVector` (`KismetMathLibrary.MakeRotator` 0.0 0.0 _returnvalue_yaw)) ActionValue_Y false)))

(event `EnhancedInput|/Game/RunOrDrown/Core/EnhancedInput/Actions/IA_RODLook`
  (params (ActionValue :type "Vector2D Structure") (ElapsedSeconds :type "Float (double-precision)") (TriggeredSeconds :type "Float (double-precision)") (InputAction :type "InputAction Object Reference" :default "/Game/RunOrDrown/Core/EnhancedInput/Actions/IA_RODLook.IA_RODLook"))
  (:`Triggered`
    (`self.AddYawInput` ActionValue_X)
    (`self.AddPitchInput` ActionValue_Y)))

(event `EnhancedInput|/Game/RunOrDrown/Core/EnhancedInput/Actions/IA_RODJump`
  (params (ActionValue :type Boolean) (ElapsedSeconds :type "Float (double-precision)") (TriggeredSeconds :type "Float (double-precision)") (InputAction :type "InputAction Object Reference" :default "/Game/RunOrDrown/Core/EnhancedInput/Actions/IA_RODJump.IA_RODJump"))
  (:`Started`
    (bind _rodplayer_character (`self.RODPlayer Character`)
      (:`then`
        (`Character.Jump` _rodplayer_character))
      (:`else`)))
  (:`Completed`
    (bind _rodplayer_character_2 (`self.RODPlayer Character`)
      (:`then`
        (`Character.StopJumping` _rodplayer_character_2))
      (:`else`))))

(event `EnhancedInput|/Game/RunOrDrown/Core/EnhancedInput/Actions/IA_RODPause`
  (params (ActionValue :type Boolean) (ElapsedSeconds :type "Float (double-precision)") (TriggeredSeconds :type "Float (double-precision)") (InputAction :type "InputAction Object Reference" :default "/Game/RunOrDrown/Core/EnhancedInput/Actions/IA_RODPause.IA_RODPause"))
  (:`Triggered`
    (if (`GameplayStatics.IsGamePaused`)
      (`GameplayStatics.SetGamePaused` false)
      (set `self.bShowMouseCursor` false)
      (bind _wbp_pause (`self.WBP_Pause`)
        (:`then`
          (`Widget.RemoveFromParent` _wbp_pause))
        (:`else`))
      (else
        (`GameplayStatics.SetGamePaused` true)
        (`self.WBP_Pause`
          (:`then`
            _)
          (:`else`
            (bind _returnvalue (`|CreateWidget` "/Game/RunOrDrown/UI/Menu/WBP_Pause.WBP_Pause_C" self))
            (bind _output_get (set `self.WBP_Pause` _returnvalue))))
        (`UserWidget.AddToViewport` _output_get 0)
        (`WidgetBlueprintLibrary.SetInputMode_GameAndUIEx` self _output_get)
        (set `self.bShowMouseCursor` true)))))

(fn `UserConstructionScript`)