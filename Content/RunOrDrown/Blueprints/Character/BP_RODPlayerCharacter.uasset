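; Player character for RunOrDrown that drowns on touching water and interacts with nearby objects.
; A water trigger overlap with BP_Water fires a one-time death that disables input, switches to UI cursor mode and ragdolls the damped mesh to fake sinking.
; Death also plays dive and drowning sounds and pushes a muffled sound mix.
; Capsule overlaps cache the current BPI_Interactable actor, which the interact input action messages.
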(event `self.ReceiveBeginPlay`
  (`GameplayStatics.ClearSoundMixModifiers`)
  (`GameplayStatics.PushSoundMixModifier` "/Game/RunOrDrown/Sounds/SCM_RODMain.SCM_RODMain"))

(event `self.WaterTrigger.OnComponentBeginOverlap`
  (params (OverlappedComponent :type "PrimitiveComponent Object Reference") (OtherActor :type "Actor Object Reference") (OtherComp :type "PrimitiveComponent Object Reference") (OtherBodyIndex :type Integer) (bFromSweep :type Boolean) (SweepResult :type "HitResult Structure (by ref)"))
  (if (`GameplayStatics.ObjectIsA` OtherActor "/Game/RunOrDrown/Blueprints/Water/BP_Water.BP_Water_C")
    (`self.OnDeath`)
    (`self.Death`)))

(event `Death`
  (bind _returnvalue (`GameplayStatics.GetPlayerController` 0))
  (bind _returnvalue_2 (`self.K2_GetActorLocation`))
  (bind _mesh (`self.Mesh`))
  (bind _linearangulardamping (`self.LinearAngularDamping`))
  (`/Engine/EditorBlueprintResources/StandardMacros.DoOnce` false
    (:`Completed`
      (`self.PhysicsON`)
      (`self.DisableInput` _returnvalue null)
      (`WidgetBlueprintLibrary.SetInputMode_UIOnlyEx` _returnvalue null)
      (set `PlayerController.bShowMouseCursor` true _returnvalue)
      ;[1 1 1] Замедялем падение, имитируя погружение в воду
      (`PrimitiveComponent.SetLinearDamping` _mesh _linearangulardamping)
      (`PrimitiveComponent.SetAngularDamping` _mesh _linearangulardamping)
      (`|ExecutionSequence`
        (:`then_0`
          ;[1 1 1] Если персонаж упал в воду, проигрываем звук нырка, а затем - звук погружения в воду
          (if (`NavMovementComponent.IsFalling` (`self.CharacterMovement`))
            (`GameplayStatics.PlaySoundAtLocation` "/Game/RunOrDrown/Sounds/FX/WAV/JumpIntoWater.JumpIntoWater" _returnvalue_2 (struct) 1.0 1.0 0.0 null null null null))
          (`GameplayStatics.PlaySoundAtLocation` "/Game/RunOrDrown/Sounds/FX/WAV/DeathInWater.DeathInWater" _returnvalue_2 (struct) 1.0 1.0 0.0 null null null null))
        (:`then_1`
          ;[1 1 1] Ставим приглушенный звук
          (`GameplayStatics.PushSoundMixModifier` "/Game/RunOrDrown/Sounds/SCM_RODDeath.SCM_RODDeath"))))))

(event `self.CapsuleComponent.OnComponentBeginOverlap`
  (params (OverlappedComponent :type "PrimitiveComponent Object Reference") (OtherActor :type "Actor Object Reference") (OtherComp :type "PrimitiveComponent Object Reference") (OtherBodyIndex :type Integer) (bFromSweep :type Boolean) (SweepResult :type "HitResult Structure (by ref)"))
  ;[1 1 1] Логика взаимодействия. Если капсула оверлапится с интерактивным объектом, нажав "Е" можно с ним взаимодействовать
  (if (`KismetSystemLibrary.DoesImplementInterface` OtherActor "/Game/RunOrDrown/Blueprints/Interfaces/BPI_Interactable.BPI_Interactable_C")
    (set `self.CurrentInteract` OtherActor)
    (set `self.bHasInteractObject` true)))

(event `self.CapsuleComponent.OnComponentEndOverlap`
  (params (OverlappedComponent :type "PrimitiveComponent Object Reference") (OtherActor :type "Actor Object Reference") (OtherComp :type "PrimitiveComponent Object Reference") (OtherBodyIndex :type Integer))
  ;[1 1 1] Логика взаимодействия. Если капсула оверлапится с интерактивным объектом, нажав "Е" можно с ним взаимодействовать
  (`self.CurrentInteract`
    (:`then`
      (set `self.CurrentInteract` null)
      (set `self.bHasInteractObject` false))
    (:`else`)))

(event `EnhancedInput|/Game/RunOrDrown/Core/EnhancedInput/Actions/IA_RODInteract`
  (params (ActionValue :type Boolean) (ElapsedSeconds :type "Float (double-precision)") (TriggeredSeconds :type "Float (double-precision)") (InputAction :type "InputAction Object Reference" :default "/Game/RunOrDrown/Core/EnhancedInput/Actions/IA_RODInteract.IA_RODInteract"))
  ;[1 1 1] Логика взаимодействия. Если капсула оверлапится с интерактивным объектом, нажав "Е" можно с ним взаимодействовать
  (:`Triggered`
    (if (`self.bHasInteractObject`)
      (bind _currentinteract (`self.CurrentInteract`)
        (:`then`
          (message `/Game/RunOrDrown/Blueprints/Interfaces/BPI_Interactable.Interact` _currentinteract))
        (:`else`)))))

(fn `PhysicsON`
  (bind _mesh (`self.Mesh`))
  (bind _capsulecomponent (`self.CapsuleComponent`))
  (`PrimitiveComponent.SetCollisionEnabled` _capsulecomponent "QueryOnly")
  (`ActorComponent.K2_DestroyComponent` _capsulecomponent)
  (`PrimitiveComponent.SetCollisionEnabled` _mesh "PhysicsOnly")
  (`PrimitiveComponent.SetSimulatePhysics` _mesh true))

(fn `UserConstructionScript`)