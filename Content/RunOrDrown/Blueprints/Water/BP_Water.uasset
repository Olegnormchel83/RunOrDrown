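; BP_Water is the water actor in RunOrDrown that rises and tints the screen when the player goes under.
; On BeginPlay it binds to the lake character's disappearance and the player's death, which enables the post-process volume.
; PlayerOnTheLake plays a sound and raises the actor by a Z offset through a timeline.
; Plane overlaps stop the rise at WaterTrigger components, while CameraCollision overlaps toggle the post-process through a FlipFlop.
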(event `self.ReceiveBeginPlay`
  (bind _returnvalue (`GameplayStatics.GetActorOfClass` "/Game/RunOrDrown/Blueprints/Character/BP_RODLakeCharacter.BP_RODLakeCharacter_C"))
  (add `/Game/RunOrDrown/Blueprints/Character/BP_RODLakeCharacter.OnDesappeared` _returnvalue (`|CreateDelegate` :!event `PlayerOnTheLake`))
  (bind _asbp_rodplayer_character (cast `/Game/RunOrDrown/Blueprints/Character/BP_RODPlayerCharacter` (`GameplayStatics.GetPlayerCharacter` 0)))
  ;[1 1 1] При всмерти меняем постпроцесс на темно-синие тона, как будто находимся под водой
  (add `/Game/RunOrDrown/Blueprints/Character/BP_RODPlayerCharacter.OnDeath` _asbp_rodplayer_character (delegate `OnPlayerDeath`)))

(event `OnPlayerDeath`
  ;[1 1 1] При всмерти меняем постпроцесс на темно-синие тона, как будто находимся под водой
  (bind _postprocessvolume (`self.PostProcessVolume`)
    (:`then`
      (set `PostProcessVolume.BlendWeight` 1.0 _postprocessvolume))
    (:`else`)))

(event `PlayerOnTheLake`
  (bind (_returnvalue_x _returnvalue_y _returnvalue_z) (`KismetMathLibrary.BreakVector` (`self.K2_GetActorLocation`)))
  (bind (_returnvalue_x_2 _returnvalue_y_2 _returnvalue_z_2) (`KismetMathLibrary.BreakVector` (`self.K2_GetActorLocation`)))
  (`GameplayStatics.PlaySoundAtLocation` "/Game/RunOrDrown/Sounds/FX/WAV/WaterSound.WaterSound" (`self.K2_GetActorLocation`) (struct) 1.0 1.0 0.0 "/Game/RunOrDrown/Sounds/Attenuation/SA_Fire.SA_Fire" null null null)
  (bind _output_get (set `self.CurrentZ` _returnvalue_z))
  (set `self.TargetZ` (+ _output_get (`self.ZOffset`)))
  (bind (_direction _zoffset) (`Timeline|Offset` :!via `PlayFromStart` :!label _label)
    (:`Update`
      (`self.K2_SetActorLocation` (`KismetMathLibrary.MakeVector` _returnvalue_x_2 _returnvalue_y_2 (`KismetMathLibrary.MapRangeClamped` _zoffset 0.0 (`self.Time`) _returnvalue_z_2 (`self.TargetZ`)))))))

(event `self.Plane1.OnComponentBeginOverlap`
  (params (OverlappedComponent :type "PrimitiveComponent Object Reference") (OtherActor :type "Actor Object Reference") (OtherComp :type "PrimitiveComponent Object Reference") (OtherBodyIndex :type Integer) (bFromSweep :type Boolean) (SweepResult :type "HitResult Structure (by ref)"))
  (if (`ActorComponent.ComponentHasTag` OtherComp "WaterTrigger")
    (goto _label :!via `Stop`)
    (elif (`ActorComponent.ComponentHasTag` OtherComp "CameraCollision")
      ;[1 1 1] Если камера окажется под водой, так же меняем постпроцесс на темно-синие тона
      (`/Engine/EditorBlueprintResources/StandardMacros.FlipFlop`
        (:`A`
          (bind _postprocessvolume (`self.PostProcessVolume`)
            (:`then`
              (set `PostProcessVolume.BlendWeight` 1.0 _postprocessvolume))
            (:`else`)))
        (:`B`
          (bind _postprocessvolume_2 (`self.PostProcessVolume`)
            (:`then`
              (set `PostProcessVolume.BlendWeight` 0.0 _postprocessvolume_2))
            (:`else`)))))))

(fn `UserConstructionScript`)