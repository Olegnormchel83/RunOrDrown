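; Jukebox actor for the final level of Run or Drown that plays the closing theme and hands the game over to the final screen.
; On BeginPlay it starts the music and a held camera fade-out on the first player's view.
; A delay matching the fade length then adds WBP_FinalWidget, disables player input, switches to UI-only mode with a mouse cursor and destroys the player character.
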(event `self.ReceiveBeginPlay`
  (bind _returnvalue (`GameplayStatics.GetPlayerController` 0))
  (bind _playercameramanager (`PlayerController.PlayerCameraManager` (`GameplayStatics.GetPlayerController` 0)))
  (`|ExecutionSequence`
    (:`then_0`
      (bind _audio (`self.Audio`)
        (:`then`
          (`AudioComponent.SetSound` _audio "/Game/RunOrDrown/Sounds/Music/WAV/FinalLevelTheme.FinalLevelTheme")
          (`AudioComponent.Play` _audio 0.0)
          (`/Engine/EditorBlueprintResources/StandardMacros.IsValid` _playercameramanager
            (:`Is Valid`
              (`PlayerCameraManager.StartCameraFade` :`self` _playercameramanager :`ToAlpha` 1.0 :`Duration` 23.5 :`bHoldWhenFinished` true))))
        (:`else`)))
    (:`then_1`
      (`KismetSystemLibrary.Delay` 23.5)
      (bind _returnvalue_2 (`|CreateWidget` "/Game/RunOrDrown/UI/Menu/WBP_FinalWidget.WBP_FinalWidget_C"))
      (`UserWidget.AddToViewport` _returnvalue_2 0)
      (`self.DisableInput` _returnvalue null)
      (`WidgetBlueprintLibrary.SetInputMode_UIOnlyEx` _returnvalue null)
      (set `PlayerController.bShowMouseCursor` true _returnvalue)
      (bind _returnvalue_3 (`GameplayStatics.GetActorOfClass` "/Game/RunOrDrown/Blueprints/Character/BP_RODPlayerCharacter.BP_RODPlayerCharacter_C"))
      (`self.K2_DestroyActor` _returnvalue_3))))

(fn `UserConstructionScript`)