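; BP_CaveTrigger is a box trigger that adjusts post-processing when the player leaves the starting cave.
; On end overlap by a Player-tagged actor, the PostprocessChange timeline plays from the start.
; Each update rebuilds the PostProcess settings, blending temperature, min/max exposure brightness and vignette toward outside-cave targets.
; The blend reads current values rather than cached starting ones, while exposure compensation and adaptation speeds are set directly.
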(event `self.Box.OnComponentEndOverlap`
  (params (OverlappedComponent :type "PrimitiveComponent Object Reference") (OtherActor :type "Actor Object Reference") (OtherComp :type "PrimitiveComponent Object Reference") (OtherBodyIndex :type Integer))
  (if (`self.ActorHasTag` OtherActor "Player")
    ;[1 1 1] Небольшие изменения в постпроцессе, когда игрок покидает начальную пещеру
    (bind _postprocess (`self.PostProcess`)
      (:`then`
        (bind (_direction _changesec) (`Timeline|PostprocessChange` :!via `PlayFromStart`)
          (:`Update`
            (bind ((`WhiteTemp` _whitetemp) (`AutoExposureMinBrightness` _autoexposureminbrightness) (`AutoExposureMaxBrightness` _autoexposuremaxbrightness) (`VignetteIntensity` _vignetteintensity)) (break `PostProcessSettings` (`PostProcessVolume.Settings` _postprocess)))
            (set `PostProcessVolume.Settings` (make `PostProcessSettings` :`TemperatureType` "TEMP_ColorTemperature" :`WhiteTemp` (`KismetMathLibrary.MapRangeClamped` _changesec 0.0 5.0 _whitetemp (`self.Temperature`)) :`AutoExposureBias` -0.5 :`AutoExposureMinBrightness` (`KismetMathLibrary.MapRangeClamped` _changesec 0.0 5.0 _autoexposureminbrightness (`self.MinExpouseOutCave`)) :`AutoExposureMaxBrightness` (`KismetMathLibrary.MapRangeClamped` _changesec 0.0 5.0 _autoexposuremaxbrightness (`self.MaxExpouseOutCave`)) :`AutoExposureSpeedUp` 0.9 :`AutoExposureSpeedDown` 0.9 :`VignetteIntensity` (`KismetMathLibrary.MapRangeClamped` _changesec 0.0 5.0 _vignetteintensity (`self.VingetteIntensity`))) _postprocess))))
      (:`else`))))

(fn `UserConstructionScript`)