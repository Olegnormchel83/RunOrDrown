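; BP_RotatingPlate is a movable plate that turns around its vertical axis when its Move event fires.
; Move calls the parent implementation, then stores the root's current rotation and a target offset in yaw by DeltaZRotate.
; The Rotate timeline restarts and maps its ZRotate track between those yaws, updating world rotation while keeping roll and pitch.
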(event `/Game/RunOrDrown/Blueprints/Interfaces/BPI_MovablePlate.Move`
  (bind _root (`self.Root`))
  (bind (_currentrotation_roll _currentrotation_pitch _currentrotation_yaw) (`KismetMathLibrary.BreakRotator` (`self.CurrentRotation`)))
  (bind (_targetrotation_roll _targetrotation_pitch _targetrotation_yaw) (`KismetMathLibrary.BreakRotator` (`self.TargetRotation`)))
  (bind (_returnvalue_roll _returnvalue_pitch) (`KismetMathLibrary.BreakRotator` (`SceneComponent.K2_GetComponentRotation` _root)))
  (`parent.Move`)
  (bind _root_2 (`self.Root`)
    (:`then`
      (bind _output_get (set `self.CurrentRotation` (`SceneComponent.K2_GetComponentRotation` _root_2)))
      (set `self.TargetRotation` (`KismetMathLibrary.MakeRotator` (.roll _output_get) (.pitch _output_get) (+ (.yaw _output_get) (`self.DeltaZRotate`))))
      (bind (_direction _zrotate) (`Timeline|Rotate` :!via `PlayFromStart`)
        (:`Update`
          (`SceneComponent.K2_SetWorldRotation` _root (`KismetMathLibrary.MakeRotator` _returnvalue_roll _returnvalue_pitch (`KismetMathLibrary.MapRangeClamped` _zrotate 0.0 1.0 _currentrotation_yaw _targetrotation_yaw)) false false))))
    (:`else`)))

(fn `UserConstructionScript`
  (`parent.UserConstructionScript`))