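; Elevator variant of a movable plate that shifts vertically each time its Move event fires.
; Move calls the parent logic, then records the Root's current world Z and adds DeltaZOffset to set the target height.
; The Offset timeline restarts from the beginning and its ZOffset track is range-mapped between the two heights, updating only Z.
; Because the target is relative to the current height, successive moves start from wherever the plate is.
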(event `/Game/RunOrDrown/Blueprints/Interfaces/BPI_MovablePlate.Move`
  (bind _root (`self.Root`))
  (bind (_returnvalue_x _returnvalue_y) (`KismetMathLibrary.BreakVector` (`SceneComponent.K2_GetComponentLocation` _root)))
  (`parent.Move`)
  (bind _root_2 (`self.Root`)
    (:`then`
      (bind (_returnvalue_x_2 _returnvalue_y_2 _returnvalue_z) (`KismetMathLibrary.BreakVector` (`SceneComponent.K2_GetComponentLocation` _root_2)))
      (bind _output_get (set `self.CurrentLocationZ` _returnvalue_z))
      (set `self.TargetLocationZ` (+ _output_get (`self.DeltaZOffset`)))
      (bind (_direction _zoffset) (`Timeline|Offset` :!via `PlayFromStart`)
        (:`Update`
          (`SceneComponent.K2_SetWorldLocation` _root (`KismetMathLibrary.MakeVector` _returnvalue_x _returnvalue_y (`KismetMathLibrary.MapRangeClamped` _zoffset 0.0 1.0 (`self.CurrentLocationZ`) (`self.TargetLocationZ`))) false false))))
    (:`else`)))

(fn `UserConstructionScript`
  (`parent.UserConstructionScript`))