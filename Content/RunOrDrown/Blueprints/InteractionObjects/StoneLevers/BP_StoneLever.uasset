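; BP_StoneLever is a one-shot interactable stone lever that triggers a linked actor.
; Its collision component shows and removes an interact hint widget as an actor tagged Player enters and leaves.
; Interact runs Push and sends MoveMessage to ControlledActor.
; Push removes the collision, slides the mesh back along local X with the HorizontalOffset timeline, then destroys the lever when the timeline finishes.
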(event `self.InteractCollision.OnComponentBeginOverlap`
  (params (OverlappedComponent :type "PrimitiveComponent Object Reference") (OtherActor :type "Actor Object Reference") (OtherComp :type "PrimitiveComponent Object Reference") (OtherBodyIndex :type Integer) (bFromSweep :type Boolean) (SweepResult :type "HitResult Structure (by ref)"))
  (if (`self.ActorHasTag` OtherActor "Player")
    (if (not (`self.bIsInViewport`))
      (bind _returnvalue (`|CreateWidget` "/Game/RunOrDrown/UI/Game/WBP_InteractHint.WBP_InteractHint_C"))
      (bind _output_get (set `self.InteractHint` _returnvalue))
      (`UserWidget.AddToViewport` _output_get 0)
      (set `self.bIsInViewport` true))))

(event `self.InteractCollision.OnComponentEndOverlap`
  (params (OverlappedComponent :type "PrimitiveComponent Object Reference") (OtherActor :type "Actor Object Reference") (OtherComp :type "PrimitiveComponent Object Reference") (OtherBodyIndex :type Integer))
  (if (`self.ActorHasTag` OtherActor "Player")
    (bind _interacthint (`self.InteractHint`)
      (:`then`
        (`Widget.RemoveFromParent` _interacthint)
        (set `self.bIsInViewport` false))
      (:`else`))))

(event `/Game/RunOrDrown/Blueprints/Interfaces/BPI_Interactable.Interact`
  (`|ExecutionSequence`
    (:`then_0`
      (`self.Push`))
    (:`then_1`
      (bind _controlledactor (`self.ControlledActor`)
        (:`then`
          (message `/Game/RunOrDrown/Blueprints/Interfaces/BPI_MovablePlate.Move` _controlledactor))
        (:`else`)))))

(event `Push`
  (bind _staticmesh (`self.StaticMesh`))
  (bind (_relativelocation_x _relativelocation_y _relativelocation_z) (`KismetMathLibrary.BreakVector` (`SceneComponent.RelativeLocation` _staticmesh)))
  (bind _interactcollision (`self.InteractCollision`)
    (:`then`
      (`ActorComponent.K2_DestroyComponent` _interactcollision)
      (bind _staticmesh_2 (`self.StaticMesh`)
        (:`then`
          (bind _relativelocation_x_2 (`KismetMathLibrary.BreakVector` (`SceneComponent.RelativeLocation` _staticmesh_2)))
          (bind _output_get (set `self.Relative Location X` _relativelocation_x_2))
          (set `self.TargetLocationX` (- _output_get 30.0))
          (bind (_direction _offset) (`Timeline|HorizontalOffset` :!via `PlayFromStart`)
            (:`Update`
              (`SceneComponent.K2_SetRelativeLocation` _staticmesh (`KismetMathLibrary.MakeVector` (`KismetMathLibrary.MapRangeClamped` _offset 0.0 1.0 (`self.Relative Location X`) (`self.TargetLocationX`)) _relativelocation_y _relativelocation_z) false false))
            (:`Finished`
              (`self.K2_DestroyActor`))))
        (:`else`)))
    (:`else`)))

(fn `UserConstructionScript`)