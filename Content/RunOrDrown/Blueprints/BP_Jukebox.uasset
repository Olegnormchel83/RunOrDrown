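; BP_Jukebox is the music player for RunOrDrown, switching between a start theme and a lake theme.
; On BeginPlay it binds to the OnDesappeared dispatcher of the BP_RODLakeCharacter found in the level, then plays StartTheme on its Audio component.
; ChangeTheme, the apparent handler for that dispatcher, stops the audio and restarts it with LakeTheme.
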(event `self.ReceiveBeginPlay`
  (`|ExecutionSequence`
    (:`then_0`
      (bind _returnvalue (`GameplayStatics.GetActorOfClass` "/Game/RunOrDrown/Blueprints/Character/BP_RODLakeCharacter.BP_RODLakeCharacter_C"))
      (add `/Game/RunOrDrown/Blueprints/Character/BP_RODLakeCharacter.OnDesappeared` _returnvalue (`|CreateDelegate` :!event `ChangeTheme`)))
    (:`then_1`
      (bind _audio (`self.Audio`)
        (:`then`
          (`AudioComponent.SetSound` _audio (`self.StartTheme`))
          (`AudioComponent.Play` _audio 0.0))
        (:`else`)))))

(event `ChangeTheme`
  (bind _audio (`self.Audio`)
    (:`then`
      (`AudioComponent.Stop` _audio)
      (`AudioComponent.SetSound` _audio (`self.LakeTheme`))
      (`AudioComponent.Play` _audio 0.0))
    (:`else`)))

(fn `UserConstructionScript`)